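; BP_GameManager is an actor that tracks the remaining bombs (BP_Obstacle actors) and a countdown timer, and displays the win state.
; On BeginPlay it records the starting obstacle count and adds a WBP_Player widget to the viewport.
; Each Tick it decrements TimeLimit, re-queries obstacles with GetAllActorsOfClass, updates the widget's texts and shows "WIN!" when none remain.
; The timer has no expiry check or lose condition.
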(event `self.ReceiveBeginPlay`
  (bind _outactors (`GameplayStatics.GetAllActorsOfClass` "/Game/Assets/Obstacles/BP_Obstacle.BP_Obstacle_C"))
  (set `self.ObstacleCount` (`KismetArrayLibrary.Array_Length` _outactors))
  (bind _returnvalue (`|CreateWidget` "/Game/WBP_Player.WBP_Player_C" (`GameplayStatics.GetPlayerController` 0)))
  (`UserWidget.AddToViewport` _returnvalue 0)
  (set `self.PlayerWidget` _returnvalue))

(event `self.ReceiveTick`
  (params (DeltaSeconds :type "Float (single-precision)"))
  (bind _gamestatus (`/Game/WBP_Player.GameStatus` (`self.PlayerWidget`)))
  (set `self.TimeLimit` (- (`self.TimeLimit`) DeltaSeconds))
  (bind _outactors (`GameplayStatics.GetAllActorsOfClass` "/Game/Assets/Obstacles/BP_Obstacle.BP_Obstacle_C"))
  (bind _returnvalue (`KismetArrayLibrary.Array_Length` _outactors))
  (if (>= _returnvalue 1)
    (`TextBlock.SetText` _gamestatus "")
    (else
      (`TextBlock.SetText` _gamestatus "WIN!")))
  (`TextBlock.SetText` (`/Game/WBP_Player.AmountLeft` (`self.PlayerWidget`)) (`KismetTextLibrary.Conv_StringToText` (`KismetStringLibrary.Concat_StrStr` "残り爆弾 - " (`KismetStringLibrary.Conv_IntToString` _returnvalue) "/" (`KismetStringLibrary.Conv_IntToString` (`self.ObstacleCount`)))))
  (`TextBlock.SetText` (`/Game/WBP_Player.TimeLimit` (`self.PlayerWidget`)) (`KismetTextLibrary.Conv_DoubleToText` (`self.TimeLimit`) "HalfToEven")))

(fn `UserConstructionScript`)