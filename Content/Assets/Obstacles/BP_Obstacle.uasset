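; BP_Obstacle is an obstacle actor that collapses through a Geometry Collection and then removes itself.
; Its Destroy function turns on physics for the Geometry Collection, turns it off for the Static Mesh, and sets IsCollapsed once.
; Tick polls that flag and, through a DoOnce, waits half a second before destroying the actor.
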(event `self.ReceiveBeginPlay`)

(event `self.ReceiveTick`
  (params (DeltaSeconds :type "Float (single-precision)"))
  (if (`self.IsCollapsed`)
    (`/Engine/EditorBlueprintResources/StandardMacros.DoOnce` false
      (:`Completed`
        (`KismetSystemLibrary.Delay` 0.5)
        (`self.K2_DestroyActor`)))))

(fn `Destroy`
  (`PrimitiveComponent.SetSimulatePhysics` (`self.GeometryCollection`) true)
  (`PrimitiveComponent.SetSimulatePhysics` (`self.StaticMesh`) false)
  (`/Engine/EditorBlueprintResources/StandardMacros.DoOnce` false
    (:`Completed`
      (set `self.IsCollapsed` true))))

(fn `UserConstructionScript`)