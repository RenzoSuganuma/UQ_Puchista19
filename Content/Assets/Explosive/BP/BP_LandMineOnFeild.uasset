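; BP_LandMineOnFeild is a land mine actor that explodes in a chain reaction with other linked explosives.
; Activate sets a one-way IsActivated flag, which Tick polls before running a one-second delay.
; After the delay it prints a debug explosion message, calls Activate on every ExplodeChain entry, then destroys itself.
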(event `self.ReceiveTick`
  (params (DeltaSeconds :type "Float (single-precision)"))
  (if (`self.IsActivated`)
    (`KismetSystemLibrary.Delay` 1.0)
    (`KismetSystemLibrary.PrintString` (`KismetStringLibrary.Concat_StrStr` (`KismetSystemLibrary.GetDisplayName` self) "Was Explode!"))
    (for _array_element (`self.ExplodeChain`)
      (`self.Activate` _array_element))
    (`self.K2_DestroyActor`)))

(fn `Activate`
  (if (not (`self.IsActivated`))
    (set `self.IsActivated` true)))

(fn `UserConstructionScript`)